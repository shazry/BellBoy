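; BP_Door is a proximity door that swings open when something enters its Sphere and closes when it leaves.
; The overlap events play or reverse a timeline that drives SMDoor's yaw, with a DoOnce playing a click at movement start and resetting when the timeline finishes.
; On BeginPlay, CurrDoorStatus sets the RectLight color for unavailable, unlocked or locked, but the status does not gate opening.
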(event `self.Sphere.OnComponentBeginOverlap`
  (params (OverlappedComponent :type "PrimitiveComponent Object Reference") (OtherActor :type "Actor Object Reference") (OtherComp :type "PrimitiveComponent Object Reference") (OtherBodyIndex :type Integer) (bFromSweep :type Boolean) (SweepResult :type "HitResult Structure (by ref)"))
  ;[1 1 1] Door Open/Close Animation (tmp component begin overlap)
  (set `self.isDoorOpen` true)
  (bind (_direction _door_animation) (`Timeline|DoorOpen Animation` :!label _label)
    (:`Update`
      (`SceneComponent.K2_SetRelativeRotation` (`self.SM_Door`) (`KismetMathLibrary.MakeRotator` 0.0 0.0 _door_animation) false false)
      (`/Engine/EditorBlueprintResources/StandardMacros.DoOnce` false :!label _label_2
        (:`Completed`
          (`GameplayStatics.PlaySoundAtLocation` "/Game/Ours/Audio/DoorClick.DoorClick" (`SceneComponent.K2_GetComponentLocation` (`self.DefaultSceneRoot`)) (struct) 1.0 1.0 0.0 null null null null))))
    (:`Finished`
      (goto _label_2 :!via `Reset`))))

(event `self.Sphere.OnComponentEndOverlap`
  (params (OverlappedComponent :type "PrimitiveComponent Object Reference") (OtherActor :type "Actor Object Reference") (OtherComp :type "PrimitiveComponent Object Reference") (OtherBodyIndex :type Integer))
  ;[1 1 1] Door Open/Close Animation (tmp component begin overlap)
  (set `self.isDoorOpen` false)
  (goto _label :!via `Reverse`))

(event `self.ReceiveBeginPlay`
  (bind _rectlight (`self.RectLight`))
  ;[1 1 1] Door Light status (tmp BeginPlay)
  (switch `/Game/Ours/Blueprints/DoorStatus` (`self.CurrDoorStatus`)
    (:`NewEnumerator2`
      (`LightComponent.SetLightColor` _rectlight (struct :`R` 0.278564 :`G` 0.328125 :`B` 0.295245 :`A` 1.0) true))
    (:`NewEnumerator0`
      (`LightComponent.SetLightColor` _rectlight (struct :`G` 0.776042 :`B` 0.075504 :`A` 1.0) true))
    (:`NewEnumerator1`
      (`LightComponent.SetLightColor` _rectlight (struct :`R` 1.0 :`G` 0.049691 :`A` 1.0) true))))

(fn `UserConstructionScript`)